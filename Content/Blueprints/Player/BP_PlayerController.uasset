(event Custom|UpdateBuildingType
  (params (BuildingType :type E_BuildingType%20Enum :default "NewEnumerator0"))
  (bind _buildingref (Variables|BuildingVariables|GetBuildingRef))
  (bind _output_get (Variables|BuildingVariables|SetBuildingSelect BuildingType))
  (switch Utilities|FlowControl|Switch|SwitchonE_BuildingType _output_get
    (:NewEnumerator0
      ;[1 1 1] Building phase stuff
      ;;[1 1 1] Sets selected building from widget input.
      (Variables|BuildingVariables|SetShownBuildingPlacement "/Game/Blueprints/Buildings/Apartment_1/BP_ApartmentPlacement.BP_ApartmentPlacement_C"))
    (:NewEnumerator1
      (Variables|BuildingVariables|SetShownBuildingPlacement "/Game/Blueprints/Buildings/Hospital/BP_HospitalPlacement.BP_HospitalPlacement_C"))
    (:NewEnumerator4
      (Variables|BuildingVariables|SetShownBuildingPlacement "/Game/Blueprints/Buildings/Cinema/BP_CinemaPlacement.BP_CinemaPlacement_C"))
    (:NewEnumerator5
      (Variables|BuildingVariables|SetShownBuildingPlacement "/Game/Blueprints/Buildings/Shop/BP_ShopPlacement.BP_ShopPlacement_C")))
  (Utilities|IsValid _buildingref
    (:Is%20Valid
      (Actor|DestroyActor _buildingref))
    (:Is%20Not%20Valid
      _))
  (CallFunction|RefreshPlaceableBuilding))

(event Custom|ToggleBuild
  (bind _gamestateref (Variables|GameState|GetGameStateRef))
  ;[1 1 1] Building phase stuff
  ;;[1 1 1] Toggle Building HUD and Input
  (Utilities|FlowControl|FlipFlop
    (:A
      (Default|SetGameState _gamestateref "NewEnumerator2")
      (CallFunction|SetBuildingMode true)
      (Variables|BuildingVariables|SetBuildKeyPressed true))
    (:B
      (Default|SetGameState _gamestateref "NewEnumerator3")
      (CallFunction|SetBuildingMode false)
      (Variables|BuildingVariables|SetBuildKeyPressed false)))
  (Utilities|ToggleBuildUI))

(event Custom|SpawnOnServer
  (params (NewParam :type Transform) (BuildingSelection :type E_BuildingType%20Enum :default "NewEnumerator0"))
  (switch Utilities|FlowControl|Switch|SwitchonE_BuildingType BuildingSelection
    (:NewEnumerator0
      (Variables|BuildingVariables|SetSpawnBuilding "/Game/Blueprints/Buildings/Apartment_1.Apartment_1_C"))
    (:NewEnumerator1
      (Variables|BuildingVariables|SetSpawnBuilding "/Game/Blueprints/Buildings/Hospital.Hospital_C"))
    (:NewEnumerator4
      (Variables|BuildingVariables|SetSpawnBuilding "/Game/Blueprints/Buildings/Cinema.Cinema_C"))
    (:NewEnumerator5
      (Variables|BuildingVariables|SetSpawnBuilding "/Game/Blueprints/Buildings/Shop.Shop_C")))
  (Game|SpawnActorfromClass (Variables|BuildingVariables|GetSpawnBuilding) NewParam "AlwaysSpawn" 0 0))

(event EventTick
  (params (DeltaSeconds :type Float%20%28single-precision%29))
  (bind _gamestateref (Variables|GameState|GetGameStateRef))
  (if (Pawn|IsLocalController)
    (Utilities|IsValid _gamestateref
      (:Is%20Valid
        (switch Utilities|FlowControl|Switch|SwitchonE_CurrentGameState (Variables|/Game/Blueprints/BP_GameState.BP_GameState_C|GetCurrentState _gamestateref)
          (:NewEnumerator2
            (CallFunction|UpdatePlacement)))))))

(event EventBeginPlay
  (if (Pawn|IsLocalController)
    (Utilities|CreatePlayerWidgets)
    (bind _asbp_game_state (Utilities|Casting|CastToBP_GameState (Game|GetGameState)))
    (Variables|GameState|SetGameStateRef _asbp_game_state)))

(event Input|ActionEvents|InputActionInteract
  (params (Key :type Key%20Structure :default "None"))
  (:Pressed
    (switch Utilities|FlowControl|Switch|SwitchonE_CurrentGameState (Variables|/Game/Blueprints/BP_GameState.BP_GameState_C|GetCurrentState (Variables|GameState|GetGameStateRef))
      (:NewEnumerator2
        (CallFunction|SpawnSelectedBuilding))
      (:NewEnumerator3
        (CallFunction|Interact)))))

(event Input|ActionEvents|InputActionToggleBuild
  (params (Key :type Key%20Structure :default "None"))
  ;[1 1 1] Building phase stuff
  ;;[1 1 1] Enters/exit build mode. TODO:: Change input to event when build phase begins.
  (:Pressed
    (CallFunction|ToggleBuild)))

(event Input|ActionEvents|InputActionMenu/Deselect
  (params (Key :type Key%20Structure :default "None"))
  (bind _self self)
  (bind _player_widget_switcher (Variables|Default|GetPlayer%20Widget%20Switcher))
  (:Pressed
    (switch Utilities|FlowControl|Switch|SwitchonE_CurrentGameState (Variables|/Game/Blueprints/BP_GameState.BP_GameState_C|GetCurrentState (Variables|GameState|GetGameStateRef))
      (:NewEnumerator0
        (Game|SetGamePaused false)
        (Default|SetGameState (Variables|GameState|GetGameStateRef) "NewEnumerator3")
        (Variables|Default|SetbShowMouseCursor false)
        (Class|WidgetSwitcher|SetActiveWidgetIndex _player_widget_switcher)
        (Input|SetInputModeGameOnly _self))
      (:NewEnumerator2
        (CallFunction|ToggleBuild))
      (:NewEnumerator3
        (Game|SetGamePaused true)
        (Default|SetGameState (Variables|GameState|GetGameStateRef) "NewEnumerator0")
        (Variables|Default|SetbShowMouseCursor true)
        (Class|WidgetSwitcher|SetActiveWidgetIndex _player_widget_switcher 1)
        (Input|SetInputModeUIOnly _self (Variables|UI|GetPauseMenuRef) "DoNotLock")))))

(fn ConstructionScript)

(fn SwitchCamera
  (Game|Player|SetViewTargetwithBlend 0 0.0 "VTBlend_Linear" 0.0 false))

(fn SetBuildingMode
  (params (CanBuild :type Boolean))
  (bind _buildingref (Variables|BuildingVariables|GetBuildingRef))
  (if (== CanBuild (Variables|BuildingVariables|GetBuildModeActive))
    (return)
    (else
      (bind _output_get (Variables|BuildingVariables|SetBuildModeActive CanBuild))
      (if _output_get
        (CallFunction|RefreshPlaceableBuilding)
        (else
          (Variables|BuildingVariables|SetShownBuildingPlacement 0)
          (Utilities|IsValid _buildingref
            (:Is%20Valid
              (Actor|DestroyActor _buildingref))))))))

(fn UpdatePlacement
  (bind _self self)
  (bind _buildingref (Variables|BuildingVariables|GetBuildingRef))
  (bind (_worldlocation _worlddirection) (Game|Player|ConvertMouseLocationToWorldSpace _self))
  (if (Variables|BuildingVariables|GetBuildModeActive)
    (bind _outhit (Collision|LineTraceByChannel _worldlocation (+ _worldlocation (* _worlddirection 7e+03)) "TraceTypeQuery3" false 0 "None"))
    (if (.bBlockingHit (Collision|BreakHitResult _outhit))
      (Utilities|IsValid _buildingref
        (:Is%20Valid
          (Rendering|SetActorHiddenInGame _buildingref false)
          (Transformation|SetActorLocation _buildingref (.Location (Collision|BreakHitResult _outhit)) false false)))
      (else
        (Utilities|IsValid _buildingref
          (:Is%20Valid
            (Rendering|SetActorHiddenInGame _buildingref true)))))
    (else
      (return))))

(fn SpawnSelectedBuilding
  (bind _buildingref (Variables|BuildingVariables|GetBuildingRef))
  (bind _returnvalue (Actor|GetComponentbyClass _buildingref "/Game/Blueprints/Components/BP_PlaceableBuildingComponent.BP_PlaceableBuildingComponent_C"))
  (if (Variables|BuildingVariables|GetBuildModeActive)
    (Utilities|IsValid _buildingref
      (:Is%20Valid
        (Utilities|IsValid _returnvalue
          (:Is%20Valid
            (if (Variables|/Game/Blueprints/Components/BP_PlaceableBuildingComponent.BP_PlaceableBuildingComponent_C|GetValidPlacement _returnvalue)
              (bind _output_get (Variables|BuildingVariables|SetCurrentBuildings (+ (Variables|BuildingVariables|GetCurrentBuildings) 1)))
              ;[1 1 1] test multi
              (if (< _output_get (Variables|BuildingVariables|GetMaxBuildings))
                (Utilities|BuildingDebugPlacementCount)
                (CallFunction|SpawnonServer (Transformation|GetActorTransform (Variables|BuildingVariables|GetBuildingRef)) (Variables|BuildingVariables|GetBuildingSelect))
                (else
                  (CallFunction|ToggleBuild)
                  (Development|PrintString "Building slots empty."))))))))
    (else
      (return))))

(fn RefreshPlaceableBuilding
  (bind _shownbuildingplacement (Variables|BuildingVariables|GetShownBuildingPlacement))
  (if (!= _shownbuildingplacement 0)
    (bind _returnvalue (Game|SpawnActorfromClass _shownbuildingplacement (Math|Transform|MakeTransform "0, 0,-10000.000000") "AlwaysSpawn" 0 0))
    (bind _output_get (Variables|BuildingVariables|SetBuildingRef _returnvalue))
    (Utilities|IsValid (Actor|GetComponentbyClass _output_get "/Game/Blueprints/Components/BP_SelectionComponent.BP_SelectionComponent_C")
      (:Is%20Valid
        (Default|InBuildingMode (Actor|GetComponentbyClass _output_get "/Game/Blueprints/Components/BP_SelectionComponent.BP_SelectionComponent_C")))
      (:Is%20Not%20Valid
        _))
    (AddComponent|AddBPPlaceableBuildingComponent (Variables|BuildingVariables|GetBuildingRef))))

(fn OnRepBuildingtoSpawn)

(fn OnRepBuildingRef)

(fn Interact
  (bind _asbp_player (Utilities|Casting|CastToBP_Player (Pawn|GetControlledPawn)))
  (bind _outhit (Collision|LineTraceByChannel (Transformation|GetWorldLocation (Variables|/Game/Blueprints/Player/BP_Player.BP_Player_C|GetPlayerCamera _asbp_player)) (+ (Transformation|GetWorldLocation (Variables|/Game/Blueprints/Player/BP_Player.BP_Player_C|GetPlayerCamera _asbp_player)) (* (Math|Vector|GetForwardVector (Transformation|GetWorldRotation (Variables|/Game/Blueprints/Player/BP_Player.BP_Player_C|GetPlayerCamera _asbp_player))) (LocalVariables|GetInteractReach))) "TraceTypeQuery1" false 0 "None"))
  (bind _asi_interactable (Utilities|Casting|CastToI_Interactable (.HitActor (Collision|BreakHitResult _outhit))))
  (Default|TriggerInterraction _asi_interactable))

(fn OnRepSpawnBuilding)