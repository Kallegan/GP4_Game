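; Player pawn with yaw-relative movement, clamped mouse-look style rotation and a hotkey for tuning trebuchet projectile mass.
; Axis inputs drive walking, strafing and controller yaw and pitch.
; Up and Down share a sphere trace around the capsule that raises or lowers a BP_TrebuchetOld projectile's mass by MassModifier and prints it.
; A disconnected camera line trace for I_Interactable remains, noted as moved to the controller.
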(event Input|AxisEvents|InputAxisLook
  (params (AxisValue :type Float%20%28single-precision%29))
  ;[1 1 1] Player Rotation
  (Pawn|Input|AddControllerPitchInput (Math|Float|Clamp(Float) AxisValue -2.0 2.0)))

(event Input|AxisEvents|InputAxisTurn
  (params (AxisValue :type Float%20%28single-precision%29))
  ;[1 1 1] Player Rotation
  (Pawn|Input|AddControllerYawInput (Math|Float|Clamp(Float) AxisValue -2.0 2.0)))

(event Input|AxisEvents|InputAxisMove
  (params (AxisValue :type Float%20%28single-precision%29))
  ;[1 1 1] Player Movement
  (Pawn|Input|AddMovementInput (Math|Vector|GetForwardVector (Math|Rotator|MakeRotator 0.0 0.0 (.Yaw (Math|Rotator|BreakRotator (Pawn|GetControlRotation :!class /Script/Engine.Pawn))))) AxisValue false))

(event Input|AxisEvents|InputAxisStrafe
  (params (AxisValue :type Float%20%28single-precision%29))
  ;[1 1 1] Player Movement
  (Pawn|Input|AddMovementInput (Math|Vector|GetRightVector (Math|Rotator|MakeRotator 0.0 0.0 (.Yaw (Math|Rotator|BreakRotator (Pawn|GetControlRotation :!class /Script/Engine.Pawn))))) AxisValue false))

(event Input|KeyboardEvents|Up
  (params (Key :type Key%20Structure))
  (bind _capsulecomponent (Variables|Collision|GetCapsuleComponent))
  (bind _massmodifier (Variables|Default|GetMassModifier))
  (bind _returnvalue (Transformation|GetWorldLocation _capsulecomponent))
  (:Pressed
    (Variables|Default|SetMoreMass true)
    (bind _outhits (Collision|MultiSphereTraceForObjects _returnvalue _returnvalue 5e+02 (Utilities|Array|MakeArray "ObjectTypeQuery2") false 0 "None"))
    (bind _array_element (Utilities|Array|ForEachLoopwithBreak _outhits :!label _label)
      (:LoopBody
        (bind _asbp_trebuchet (Utilities|Casting|CastToBP_TrebuchetOld (.HitActor (Collision|BreakHitResult _array_element))))
        (if (Variables|Default|GetMoreMass)
          (Class|PrimitiveComponent|SetMassOverrideinKg (Variables|/Game/Blueprints/BP_TrebuchetOld.BP_TrebuchetOld_C|GetSM_Projectile _asbp_trebuchet) "None" (+ (Physics|GetMass (Variables|/Game/Blueprints/BP_TrebuchetOld.BP_TrebuchetOld_C|GetSM_Projectile _asbp_trebuchet)) _massmodifier) true)
          (else
            (Class|PrimitiveComponent|SetMassOverrideinKg (Variables|/Game/Blueprints/BP_TrebuchetOld.BP_TrebuchetOld_C|GetSM_Projectile _asbp_trebuchet) "None" (- (Physics|GetMass (Variables|/Game/Blueprints/BP_TrebuchetOld.BP_TrebuchetOld_C|GetSM_Projectile _asbp_trebuchet)) _massmodifier) true)))
        (Development|PrintString (Utilities|String|ToString(Float) (Physics|GetMass (Variables|/Game/Blueprints/BP_TrebuchetOld.BP_TrebuchetOld_C|GetSM_Projectile _asbp_trebuchet))))
        (goto _label Break)))))

(event Input|KeyboardEvents|Down
  (params (Key :type Key%20Structure))
  (bind _capsulecomponent (Variables|Collision|GetCapsuleComponent))
  (bind _massmodifier (Variables|Default|GetMassModifier))
  (bind _returnvalue (Transformation|GetWorldLocation _capsulecomponent))
  (:Pressed
    (Variables|Default|SetMoreMass false)
    (bind _outhits (Collision|MultiSphereTraceForObjects _returnvalue _returnvalue 5e+02 (Utilities|Array|MakeArray "ObjectTypeQuery2") false 0 "None"))
    (bind _array_element (Utilities|Array|ForEachLoopwithBreak _outhits :!label _label)
      (:LoopBody
        (bind _asbp_trebuchet (Utilities|Casting|CastToBP_TrebuchetOld (.HitActor (Collision|BreakHitResult _array_element))))
        (if (Variables|Default|GetMoreMass)
          (Class|PrimitiveComponent|SetMassOverrideinKg (Variables|/Game/Blueprints/BP_TrebuchetOld.BP_TrebuchetOld_C|GetSM_Projectile _asbp_trebuchet) "None" (+ (Physics|GetMass (Variables|/Game/Blueprints/BP_TrebuchetOld.BP_TrebuchetOld_C|GetSM_Projectile _asbp_trebuchet)) _massmodifier) true)
          (else
            (Class|PrimitiveComponent|SetMassOverrideinKg (Variables|/Game/Blueprints/BP_TrebuchetOld.BP_TrebuchetOld_C|GetSM_Projectile _asbp_trebuchet) "None" (- (Physics|GetMass (Variables|/Game/Blueprints/BP_TrebuchetOld.BP_TrebuchetOld_C|GetSM_Projectile _asbp_trebuchet)) _massmodifier) true)))
        (Development|PrintString (Utilities|String|ToString(Float) (Physics|GetMass (Variables|/Game/Blueprints/BP_TrebuchetOld.BP_TrebuchetOld_C|GetSM_Projectile _asbp_trebuchet))))
        (goto _label Break)))))

(fn ConstructionScript)