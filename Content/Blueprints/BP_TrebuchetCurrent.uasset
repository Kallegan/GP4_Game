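; Physics-driven trebuchet that players reload, fire and rotate by overlapping its collision boxes.
; Firing enables simulation on arm, weight and projectile plus wind, and a per-tick dot-product check breaks the rope constraint at the release point.
; Projectile hits sphere-trace to damage BP_Building actors, spawn a directional FS_ExplodeField_Explosion for destruction and scale down projectile velocity.
; Reloading re-parents and resets the simulated parts, then reattaches the projectile to the rope.
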(event OnComponentHit(SM_Projectile)
  (params (HitComponent :type Primitive%20Component%20Object%20Reference) (OtherActor :type Actor%20Object%20Reference) (OtherComp :type Primitive%20Component%20Object%20Reference) (NormalImpulse :type Vector :default "0, 0, 0") (Hit :type Hit%20Result%20Structure%20%28by%20ref%29))
  (bind _damagedbuildings (Variables|Default|GetDamagedBuildings))
  (bind _sm_projectile (Variables|Default|GetSM_Projectile))
  (Utilities|Casting|CastToBP_TrebuchetCurrent OtherActor
    (:CastFailed
      ;[1 1 1] WIND
      (Default|EnableorDisableWind (Variables|Default|GetBP_WindComponent) false)
      (if (Variables|ProjectileDamage|GetRequireBuildingHIt)
        (if (Variables|ProjectileDamage|GetCanDoDamageAfterBounce)
          (Utilities|Casting|CastToBP_Building OtherActor)
          (else
            (Utilities|Casting|CastToBP_Building OtherActor
              (:then
                _)
              (:CastFailed
                (bind _output_get (Variables|ProjectileDamage|SetCanDoDamage false)))))))
      (if _output_get
        (bind _outhits (Collision|MultiSphereTraceForObjects (.location Hit) (.location Hit) (Variables|ProjectileDamage|GetRadius) (Utilities|Array|MakeArray "ObjectTypeQuery7") false 0 (Variables|ProjectileDamage|GetDraw%20Debug%20Type) true "(R=1.000000,G=0.000000,B=0.000000,A=1.000000)" "(R=0.000000,G=1.000000,B=0.000000,A=1.000000)" (Variables|ProjectileDamage|GetDraw%20Time)))
        (for (_array_element _array_index) _outhits
          (if (Utilities|IsValid (.HitActor (Collision|BreakHitResult _array_element)))
            (bind _asbp_building (Utilities|Casting|CastToBP_Building (.HitActor (Collision|BreakHitResult _array_element))))
            (if (not (Utilities|Array|ContainsItem _damagedbuildings _asbp_building))
              (Default|TakeDamage _asbp_building (Variables|ProjectileDamage|GetDamage))
              (Utilities|Array|Insert _damagedbuildings _asbp_building _array_index))))
        (bind _returnvalue (Game|SpawnActorfromClass "/Game/GeometryCollections/FS_ExplodeField_Explosion.FS_ExplodeField_Explosion_C" (Math|Transform|MakeTransform (.location Hit) "0, 0, 0" "1.000000,1.000000,1.000000") "Undefined" 0 0))
        (Default|SetExplosionDirection _returnvalue (Variables|ProjectileDamage|GetDirectional%20Magnitude) (* (Math|Vector|Normalize (Transformation|GetComponentVelocity HitComponent)) "-1.000000,-1.000000,1.000000"))
        (Default|SetExplosionRadialMagnitude _returnvalue (Variables|ProjectileDamage|GetRadial%20Magnitude))
        (Default|SetExplodeRadius _returnvalue (Variables|ProjectileDamage|GetRadius))
        (Default|SetExplosionStrainMagnitude _returnvalue (Variables|ProjectileDamage|GetStrain%20Magnitude))
        (Default|Explode _returnvalue)
        (Variables|ProjectileDamage|SetCanDoDamage false)
        (Utilities|Array|Clear _damagedbuildings))
      (Physics|SetPhysicsLinearVelocity _sm_projectile (* (Transformation|GetComponentVelocity _sm_projectile) (Variables|ProjectileDamage|GetVelocityReductionAfterHit)) false "None"))))

(event OnComponentBeginOverlap(ReloadCollisionBox)
  (params (OverlappedComponent :type Primitive%20Component%20Object%20Reference) (OtherActor :type Actor%20Object%20Reference) (OtherComp :type Primitive%20Component%20Object%20Reference) (OtherBodyIndex :type Integer) (bFromSweep :type Boolean) (SweepResult :type Hit%20Result%20Structure%20%28by%20ref%29))
  (if (not (Variables|TrebuchetSettings|GetbIsLoaded))
    (Utilities|Casting|CastToBP_Player OtherActor)
    (Utilities|FlowControl|DoOnce false
      (:Completed
        (CallFunction|ReloadServer)
        (bind _pull_lever (Timeline|Timeline_0 Play)
          (:Update
            (Transformation|SetRelativeRotation (Variables|Default|GetSM_Lever_Handle) (Math|Rotator|MakeRotator (* _pull_lever 9e+01) 0.0 0.0) false false)
            (Utilities|FlowControl|DoOnce false) ; enters at Reset
          ))))))

(event OnComponentBeginOverlap(FireCollisionBox)
  (params (OverlappedComponent :type Primitive%20Component%20Object%20Reference) (OtherActor :type Actor%20Object%20Reference) (OtherComp :type Primitive%20Component%20Object%20Reference) (OtherBodyIndex :type Integer) (bFromSweep :type Boolean) (SweepResult :type Hit%20Result%20Structure%20%28by%20ref%29))
  (if (Variables|TrebuchetSettings|GetbIsLoaded)
    (Utilities|Casting|CastToBP_Player OtherActor)
    (Utilities|FlowControl|DoOnce false
      (:Completed
        (CallFunction|FireServer)
        (bind _pull_lever (Timeline|Timeline_1 Play)
          (:Update
            (Transformation|SetRelativeRotation (Variables|Default|GetSM_Lever_Handle1) (Math|Rotator|MakeRotator 0.0 (* _pull_lever -9e+01) 0.0) false false)
            (Utilities|FlowControl|DoOnce false) ; enters at Reset
          ))))))

(event OnComponentBeginOverlap(Collision_RotaionHandle)
  (params (OverlappedComponent :type Primitive%20Component%20Object%20Reference) (OtherActor :type Actor%20Object%20Reference) (OtherComp :type Primitive%20Component%20Object%20Reference) (OtherBodyIndex :type Integer) (bFromSweep :type Boolean) (SweepResult :type Hit%20Result%20Structure%20%28by%20ref%29))
  ;[1 1 1] Rotate Trebuchet
  (Utilities|Casting|CastToBP_Player OtherActor)
  (Utilities|IsValid (Variables|Default|GetRotationSound)
    (:Is%20Valid
      (Class|AudioComponent|SetPaused (Variables|Default|GetRotationSound) false))
    (:Is%20Not%20Valid
      _))
  (if (<= (Math|Vector|DotProduct (Math|Vector|Normalize (- (Transformation|GetWorldLocation (Variables|/Script/Engine.Actor|GetRootComponent OtherActor)) (Transformation|GetWorldLocation (Variables|Default|GetSM_RotationHandle)))) (Math|Vector|GetRightVector (Variables|Default|GetSM_RotationHandle))) 0.0)
    (Variables|/Script/Engine.RotatingMovementComponent|SetRotationRate (Variables|Default|GetRotatingMovement) (Math|Rotator|MakeRotator 0.0 0.0 (Math|Conversions|ToFloat(Integer) (Variables|TrebuchetSettings|GetRotation%20Speed))))
    (else
      (Variables|/Script/Engine.RotatingMovementComponent|SetRotationRate (Variables|Default|GetRotatingMovement) (Math|Rotator|MakeRotator 0.0 0.0 (Math|Conversions|ToFloat(Integer) (* (Variables|TrebuchetSettings|GetRotation%20Speed) -1)))))))

(event OnComponentEndOverlap(Collision_RotaionHandle)
  (params (OverlappedComponent :type Primitive%20Component%20Object%20Reference) (OtherActor :type Actor%20Object%20Reference) (OtherComp :type Primitive%20Component%20Object%20Reference) (OtherBodyIndex :type Integer))
  (bind _rotationsound (Variables|Default|GetRotationSound))
  ;[1 1 1] Rotate Trebuchet
  (Utilities|Casting|CastToBP_Player OtherActor)
  (Variables|/Script/Engine.RotatingMovementComponent|SetRotationRate (Variables|Default|GetRotatingMovement) "0, 0, 0")
  (Utilities|IsValid _rotationsound
    (:Is%20Valid
      (Class|AudioComponent|SetPaused _rotationsound true))))

(event Custom|Activate%20Physic%20Simulation
  ;[1 1 1] Toggle Physic Simulation
  (Physics|SetSimulatePhysics (Variables|Default|GetSM_Trebuchet_Weight) true))

(event Custom|Dissable%20Physic%20Simulation
  ;[1 1 1] Toggle Physic Simulation
  (Physics|SetSimulatePhysics (Variables|Default|GetSM_Trebuchet_Weight) false))

(event Custom|ReloadServer
  (CallFunction|ReloadProjectile))

(event Custom|AttatchProjectile
  ;[1 1 1] Attatch/Detatch Projectile
  (Variables|ProjectileDamage|SetCanDoDamage true)
  (Class|CableComponent|SetAttachEndtoComponent (Variables|Default|GetRope) (Variables|Default|GetSM_Projectile) "None")
  (Class|PhysicsConstraintComponent|SetConstrainedComponents (Variables|Default|GetPhysicsConstraint_Rope) (Variables|Default|GetSM_Trebuchet_Arm) "" (Variables|Default|GetSM_Projectile) "None"))

(event Custom|DetatchProjectile
  ;[1 1 1] Attatch/Detatch Projectile
  (Class|CableComponent|SetAttachEndtoComponent (Variables|Default|GetRope) 0 "None")
  (Class|PhysicsConstraintComponent|BreakConstraint (Variables|Default|GetPhysicsConstraint_Rope)))

(event Custom|FireProjectile
  ;[1 1 1] Fire/Reload
  ;;[1 1 1] Fire Projectile
  (if (Variables|TrebuchetSettings|GetbIsLoaded)
    (Variables|TrebuchetSettings|SetbIsLoaded false)
    (CallFunction|ActivatePhysicSimulation)
    (Audio|PlaySoundatLocation "/Game/SFX/FireTrebuchet.FireTrebuchet" (Transformation|GetActorLocation) "0, 0, 0" 1.0 1.0 0.0 0 0 0 0)
    ;;;[1 1 1] WIND
    (Default|EnableorDisableWind (Variables|Default|GetBP_WindComponent) true)))

(event Custom|ReloadProjectile
  ;[1 1 1] Fire/Reload
  ;;[1 1 1] Load Projectile
  ;;;[1 1 1] WIND
  (Default|EnableorDisableWind (Variables|Default|GetBP_WindComponent) false :!label _label)
  (if (not (Variables|TrebuchetSettings|GetbIsLoaded))
    (Variables|TrebuchetSettings|SetbIsLoaded true)
    (CallFunction|ResetTransform)
    (CallFunction|AttatchProjectile)
    (Audio|PlaySoundatLocation "/Game/SFX/ReloadTrebuchet.ReloadTrebuchet" (Transformation|GetWorldLocation (Variables|Default|GetRope)) "0, 0, 0" 1.0 1.0 0.0 0 0 0 0)
    ;;;[1 1 1] WIND
    (Default|SetupWind (Variables|Default|GetBP_WindComponent) (Variables|Default|GetSM_Projectile))
    (goto _label)))

(event Custom|CheckReleasePoint
  (if (<= (Math|Vector|DotProduct (Math|Vector|Normalize (- (Transformation|GetWorldLocation (Variables|Default|GetReleasePoint)) (Transformation|GetWorldLocation (Variables|Default|GetSM_Projectile)))) (Math|Vector|GetForwardVector (Variables|Default|GetReleasePoint))) 0.0)
    (CallFunction|DetatchProjectile)))

(event Custom|FireServer
  (CallFunction|FireProjectile))

(event EventTick
  (params (DeltaSeconds :type Float%20%28single-precision%29))
  (CallFunction|CheckReleasePoint))

(event EventBeginPlay
  ;[1 1 1] WIND
  (Default|SetupWind (Variables|Default|GetBP_WindComponent) (Variables|Default|GetSM_Projectile))
  (bind _returnvalue (Audio|SpawnSoundAttached "/Game/SFX/PushTrebuchet.PushTrebuchet" (Variables|Default|GetSM_Trebuchet_Base) "None" "0, 0, 0" "0, 0, 0" "KeepRelativeOffset" false 1.0 1.0 0.0 0 0))
  (bind _output_get (Variables|Default|SetRotationSound _returnvalue))
  (Utilities|IsValid _output_get
    (:Is%20Valid
      (Class|AudioComponent|SetPaused _output_get true))))

(fn ConstructionScript)

(fn ParentComponents
  ;[1 1 1] Attatch Arm (Re-Parent)
  (Transformation|AttachComponentToComponent (Variables|Default|GetPhysicsConstraint_Rope) (Variables|Default|GetRope) "None" "KeepWorld" "KeepWorld" "KeepRelative" true)
  (Transformation|AttachComponentToComponent (Variables|Default|GetRope) (Variables|Default|GetSM_Trebuchet_Arm) "None" "KeepWorld" "KeepWorld" "KeepRelative" true)
  (Transformation|AttachComponentToComponent (Variables|Default|GetSM_Trebuchet_Arm) (Variables|Default|GetSM_Trebuchet_Base) "None" "KeepWorld" "KeepWorld" "KeepRelative" true)
  (Transformation|AttachComponentToComponent (Variables|Default|GetPhysicsConstraint_Arm) (Variables|Default|GetSM_Trebuchet_Arm) "None" "KeepWorld" "KeepWorld" "KeepRelative" true)
  ;[1 1 1] Attatch Weight (Re-Parent)
  (Transformation|AttachComponentToComponent (Variables|Default|GetPhysicsConstraint_Weight) (Variables|Default|GetSM_Trebuchet_Weight) "None" "KeepWorld" "KeepWorld" "KeepRelative" true)
  (Transformation|AttachComponentToComponent (Variables|Default|GetSM_Trebuchet_Weight) (Variables|Default|GetSM_Trebuchet_Base) "None" "KeepWorld" "KeepWorld" "KeepRelative" true)
  ;[1 1 1] Attach Projectile (Re-Parent)
  (Transformation|AttachComponentToComponent (Variables|Default|GetSM_Projectile) (Variables|Default|GetSM_Trebuchet_Base) "None" "KeepWorld" "KeepWorld" "KeepRelative" true))

(fn ResetTransform
  ;[1 1 1] Reset Position/Rotation
  (CallFunction|ParentComponents)
  (Transformation|SetRelativeLocationAndRotation (Variables|Default|GetSM_Trebuchet_Arm) "0, 0,950.000000" "135.000000,0.000000, 0" false false)
  (Transformation|SetRelativeLocationAndRotation (Variables|Default|GetSM_Trebuchet_Weight) "240.000000, 0,1190.000000" "0, 0, 0" false false)
  (Transformation|SetRelativeLocationAndRotation (Variables|Default|GetSM_Projectile) "-150.000000, 0,80.000000" "0, 0, 0" false false))