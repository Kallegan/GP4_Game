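; An actor component that makes its owner, apparently a building, highlightable on hover and selectable by click.
; On BeginPlay it binds the owner's click event and, if a static mesh component exists, caches it and binds cursor-over events that toggle custom depth rendering.
; Each click flips the Targeted flag and swaps the mesh's first material between green and red.
; A temporary InBuildingMode event destroys the component.
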(event Custom|OnMouseClicked
  (params (TouchedActor :type Actor%20Object%20Reference) (ButtonPressed :type Key%20Structure :default "None"))
  (bind _staticmeshref (Variables|Default|GetStaticMeshRef))
  (Variables|Default|SetTargeted (not (Variables|Default|GetTargeted)))
  (Utilities|IsValid (Variables|Default|GetStaticMeshRef)
    (:Is%20Valid
      (if (Variables|Default|GetTargeted)
        (Rendering|Material|SetMaterial _staticmeshref 0 "/AnimationSharing/AnimSharingGreen.AnimSharingGreen")
        (else
          (Rendering|Material|SetMaterial _staticmeshref 0 "/AnimationSharing/AnimSharingRed.AnimSharingRed"))))))

(event Custom|MouseHoverBegins
  (params (TouchedActor :type Actor%20Object%20Reference))
  (Rendering|SetRenderCustomDepth (Variables|Default|GetStaticMeshRef) true))

(event Custom|MouseHoverEnds
  (params (TouchedActor :type Actor%20Object%20Reference))
  (Rendering|SetRenderCustomDepth (Variables|Default|GetStaticMeshRef) false))

(event Custom|CustomEvent_0
  (Rendering|SetRenderCustomDepth (Variables|Default|GetStaticMeshRef) false))

(event Custom|InBuildingMode
  ;[1 1 1] TEMP
  (Components|DestroyComponent))

(event EventBeginPlay
  (bind _returnvalue (Components|GetOwner))
  (bind _returnvalue_2 (Components|GetOwner))
  (bind _returnvalue_3 (Actor|GetComponentbyClass _returnvalue_2 "/Script/Engine.StaticMeshComponent"))
  (EventDispatchers|BindEventtoOnClicked _returnvalue_2 (delegate Custom|OnMouseClicked))
  (Utilities|IsValid _returnvalue_3
    (:Is%20Valid
      (Variables|Default|SetStaticMeshRef _returnvalue_3)
      (EventDispatchers|BindEventtoOnBeginCursorOver _returnvalue (delegate Custom|MouseHoverBegins))
      (EventDispatchers|BindEventtoOnEndCursorOver _returnvalue (delegate Custom|MouseHoverEnds)))))