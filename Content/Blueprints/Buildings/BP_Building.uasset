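; BP_Building is a destructible building that tracks health and collapses through a Chaos Geometry Collection.
; Damage lowers CurrentHealth and plays the BuildingDestroyed sound on every hit; at zero health, physics simulation is enabled on the collection.
; The first Chaos break event unbinds itself, prints the building type as destroyed and removes the static mesh component.
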(event Custom|TakeDamage
  (params (Damage :type Float%20%28double-precision%29))
  (Audio|SpawnSoundatLocation "/Game/SFX/BuildingDestroyed.BuildingDestroyed" (Transformation|GetActorLocation self) "0, 0, 0" 1.0 1.0 0.0 0 0)
  (CallFunction|SetCurrentHealth (- (Variables|Default|GetCurrentHealth) Damage)))

(event Custom|SetCurrentHealth
  (params (Health :type Float%20%28double-precision%29))
  (bind _output_get (Variables|Default|SetCurrentHealth Health))
  (if (<= _output_get 0.0)
    (CallFunction|EnableSimulatePhysics)))

(event Custom|EnableSimulatePhysics
  (Physics|SetSimulatePhysics (stale EventBeginPlay _output_get) true))

(event Custom|BreakEvent
  (params (BreakEvent :type Chaos%20Break%20Event%20Structure%20%28by%20ref%29))
  (EventDispatchers|UnbindEventfromOnChaosBreakEvent (stale EventBeginPlay _output_get) (delegate Custom|BreakEvent))
  (Development|PrintString (Utilities|String|Append (Utilities|String|MakeLiteralString (Utilities|String|EnumtoString (Variables|Default|GetBuildingType))) (Utilities|String|MakeLiteralString " destroyed!")))
  (Components|DestroyComponent (Actor|GetComponentbyClass "/Script/Engine.StaticMeshComponent")))

(event EventBeginPlay
  (CallFunction|SetCurrentHealth (Variables|Default|GetHealth))
  (bind _output_get (Variables|Default|SetGeoCollection (Actor|GetComponentbyClass "/Script/GeometryCollectionEngine.GeometryCollectionComponent")))
  (Class|GeometryCollectionComponent|SetNotifyBreaks _output_get true)
  (EventDispatchers|AssignOnChaosBreakEvent _output_get (delegate Custom|BreakEvent))
  (if true
    _))

(fn ConstructionScript)